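; Mortar Blueprint that sets up an aimable, fireable tank-style weapon with a health bar widget.
; On BeginPlay it initialises the TankAiming component with its barrel and turret, then passes itself to the HealthBar widget as its TankHealth source.
; The Fire input action calls TankAiming to fire.
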(event Collision|EventActorBeginOverlap
  (params (OtherActor :type Actor%20Object%20Reference)))

(event EventBeginPlay
  (Class|TankAimingComponent|Initialise (Variables|Default|GetTankAiming) (Variables|Default|GetTankBarrel) (Variables|Default|GetTankTurret))
  (bind _ashealth_bar (Utilities|Casting|CastToHealthBar (UserInterface|GetUserWidgetObject (Variables|Default|GetWidget))))
  (Variables|/Game/UI/HealthBar.HealthBar_C|SetTankHealth _ashealth_bar self))

(event EventTick
  (params (DeltaSeconds :type Float%20%28single-precision%29)))

(event Input|ActionEvents|InputActionFire
  (params (Key :type Key%20Structure :default "AnyKey"))
  ;[1 1 1] Fire
  (:Pressed
    (Class|TankAimingComponent|Fire (Variables|Default|GetTankAiming))))

(fn ConstructionScript)